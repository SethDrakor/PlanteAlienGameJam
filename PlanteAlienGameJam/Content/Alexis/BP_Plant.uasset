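; BP_Plant is a destructible plant pickup that awards score when an actor tagged Player overlaps it.
; It plays a sound on spawn and caches the VehiclePlayerController for player 0.
; The PlantCollision overlap adds ScorePoints and decrements PlantAlive on that controller, plays a scream, then destroys the plant.
; The Destroyed event adds a swoosh sound and a particle burst at the plant's location.
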(event `self.ReceiveBeginPlay`
  (`GameplayStatics.PlaySoundAtLocation` "/Game/Alexis/the-gremlin-audio-test.the-gremlin-audio-test" (`self.K2_GetActorLocation`) (struct) 1.0 1.0 0.0 null null null null)
  ;[1 1 1] Get Player Controller
  (bind _asvehicle_player_controller (cast `/Game/VehicleTemplate/Blueprints/VehiclePlayerController` (`GameplayStatics.GetPlayerController` 0)))
  (set `self.PlayerController` _asvehicle_player_controller))

(event `self.PlantCollision.OnComponentBeginOverlap`
  (params (OverlappedComponent :type "PrimitiveComponent Object Reference") (OtherActor :type "Actor Object Reference") (OtherComp :type "PrimitiveComponent Object Reference") (OtherBodyIndex :type Integer) (bFromSweep :type Boolean) (SweepResult :type "HitResult Structure (by ref)"))
  ;[1 1 1] Destruction on Collision
  (if (`self.ActorHasTag` OtherActor "Player")
    (`/Game/VehicleTemplate/Blueprints/VehiclePlayerController.AddPlayerScore` (`self.PlayerController`) (`self.ScorePoints`))
    (set `/Game/VehicleTemplate/Blueprints/VehiclePlayerController.PlantAlive` (- (`/Game/VehicleTemplate/Blueprints/VehiclePlayerController.PlantAlive` (`self.PlayerController`)) 1) (`self.PlayerController`))
    (`GameplayStatics.PlaySoundAtLocation` "/Game/Alexis/scream-sound-effect-terrifying.scream-sound-effect-terrifying" (`self.K2_GetActorLocation`) (struct) 1.0 1.0 0.0 null null null null)
    (`self.K2_DestroyActor`)))

(event `self.ReceiveDestroyed`
  ;[1 1 1] Spawn Feedbacks on Destruction
  (`GameplayStatics.PlaySoundAtLocation` "/Game/Alexis/WAV_Swoosh.WAV_Swoosh" (`self.K2_GetActorLocation`) (struct) 1.0 1.0 0.0 null null null null)
  (`GameplayStatics.SpawnEmitterAtLocation` "/Game/FXVarietyPack/Particles/P_ky_ThunderBallHit.P_ky_ThunderBallHit" (`self.K2_GetActorLocation`)))

(fn `UserConstructionScript`)